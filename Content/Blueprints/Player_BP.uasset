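; Player Blueprint that handles axis-driven movement and a placeholder interact action.
; MoveUp and MoveRight feed movement input along the actor's up and right vectors, and BeginPlay applies one upward input after a short delay.
; Interact only prints the actor's display name.
; A SetInteract event stores a CanInteract flag, which these graphs never read.
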(event `self.ReceiveBeginPlay`
  (`KismetSystemLibrary.Delay` 0.1)
  (`self.AddMovementInput` (`self.GetActorUpVector`)))

(event `InputAxis|MoveUp`
  (params (AxisValue :type "Float (single-precision)"))
  (`self.AddMovementInput` (`self.GetActorUpVector`) AxisValue))

(event `InputAxis|MoveRight`
  (params (AxisValue :type "Float (single-precision)"))
  (`self.AddMovementInput` (`self.GetActorRightVector`) AxisValue))

(event `InputAction|Interact`
  (params (Key :type "Key Structure"))
  (:`Pressed`
    (`KismetSystemLibrary.PrintString` (`KismetSystemLibrary.GetDisplayName` null))))

(event `SetInteract`
  (params (CanInteract :type Boolean))
  (set `self.CanInteract` CanInteract))

(fn `UserConstructionScript`)